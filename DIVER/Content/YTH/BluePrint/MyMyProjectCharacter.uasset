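; Character Blueprint that switches the player between walking and swimming and tracks breathing around water areas marked by Trigger Volumes.
; The CheckSwimCollider overlap toggles movement mode, the current physics volume's water flag and IsSwimming, zeroing vertical velocity on entry and all velocity on exit.
; A separate CheckBreath collider clears IsBreathing inside a Trigger Volume and restores it on leaving.
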(event `StartSwimming`
  (bind _charactermovement (`self.CharacterMovement`))
  (bind (_velocity_x _velocity_y) (`KismetMathLibrary.BreakVector` (`MovementComponent.Velocity` _charactermovement)))
  (set `MovementComponent.Velocity` (`KismetMathLibrary.MakeVector` _velocity_x _velocity_y) _charactermovement)
  (`CharacterMovementComponent.SetMovementMode` _charactermovement "MOVE_Swimming" 0)
  (set `PhysicsVolume.bWaterVolume` true (`MovementComponent.GetPhysicsVolume` (`self.CharacterMovement`)))
  (set `self.isSwimming` true))

(event `StopSwimming`
  (bind _charactermovement (`self.CharacterMovement`))
  (`CharacterMovementComponent.SetMovementMode` _charactermovement "MOVE_Walking" 0)
  (set `MovementComponent.Velocity` (0.0 0.0 0.0) _charactermovement)
  (set `PhysicsVolume.bWaterVolume` false (`MovementComponent.GetPhysicsVolume` _charactermovement))
  (set `self.isSwimming` false))

(event `self.CheckSwimCollider.OnComponentBeginOverlap`
  (params (OverlappedComponent :type "PrimitiveComponent Object Reference") (OtherActor :type "Actor Object Reference") (OtherComp :type "PrimitiveComponent Object Reference") (OtherBodyIndex :type Integer) (bFromSweep :type Boolean) (SweepResult :type "HitResult Structure (by ref)"))
  (cast `TriggerVolume` OtherActor)
  (`self.StartSwimming`))

(event `self.CheckSwimCollider.OnComponentEndOverlap`
  (params (OverlappedComponent :type "PrimitiveComponent Object Reference") (OtherActor :type "Actor Object Reference") (OtherComp :type "PrimitiveComponent Object Reference") (OtherBodyIndex :type Integer))
  (cast `TriggerVolume` OtherActor)
  (`self.StopSwimming`))

(event `self.CheckBreath.OnComponentBeginOverlap`
  (params (OverlappedComponent :type "PrimitiveComponent Object Reference") (OtherActor :type "Actor Object Reference") (OtherComp :type "PrimitiveComponent Object Reference") (OtherBodyIndex :type Integer) (bFromSweep :type Boolean) (SweepResult :type "HitResult Structure (by ref)"))
  (cast `TriggerVolume` OtherActor)
  (set `self.isBreathing` false))

(event `self.CheckBreath.OnComponentEndOverlap`
  (params (OverlappedComponent :type "PrimitiveComponent Object Reference") (OtherActor :type "Actor Object Reference") (OtherComp :type "PrimitiveComponent Object Reference") (OtherBodyIndex :type Integer))
  (cast `TriggerVolume` OtherActor)
  (set `self.isBreathing` true))

(fn `UserConstructionScript`)